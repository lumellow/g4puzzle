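; Door Blueprint that swings open when an overlap enters its trigger box, optionally locked until every key in the level is found.
; On BeginPlay it binds to each KeyActorClass actor's key-found event and counts them, or starts unlocked if no key class is set.
; Once all keys are found, overlaps play a timeline that yaws the hinge 90 degrees, reversed on end overlap.
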(event OnComponentBeginOverlap(Box)
  (params (OverlappedComponent :type Primitive%20Component%20Object%20Reference) (OtherActor :type Actor%20Object%20Reference) (OtherComp :type Primitive%20Component%20Object%20Reference) (OtherBodyIndex :type Integer) (bFromSweep :type Boolean) (SweepResult :type Hit%20Result%20Structure%20%28by%20ref%29))
  (if (Variables|Default|GetCanOpen)
    (CallFunction|OpenDoor)))

(event OnComponentEndOverlap(Box)
  (params (OverlappedComponent :type Primitive%20Component%20Object%20Reference) (OtherActor :type Actor%20Object%20Reference) (OtherComp :type Primitive%20Component%20Object%20Reference) (OtherBodyIndex :type Integer))
  (CallFunction|CloseDoor))

(event Custom|KeyFound
  (bind _result (Math|Integer|IncrementInt (Variables|Default|GetFoundKeys))
    (:%20%20
      (if (>= _result (Variables|Default|GetTotalKeys))
        (Variables|Default|SetCanOpen true)
        (else
          (Variables|Default|SetCanOpen false))))))

(event Custom|OpenDoor
  ;[0.4271 0.4927 1] Open and close door
  (bind _opendoor (Timeline|Timeline_Door Play)
    (:Update
      (Transformation|SetRelativeRotation (Variables|Default|GetDoorHinge) (Math|Rotator|MakeRotator 0.0 0.0 (Math|Float|Lerp 0.0 9e+01 _opendoor)) false false))))

(event Custom|CloseDoor
  ;[0.4271 0.4927 1] Open and close door
  (bind _opendoor (Timeline|Timeline_Door Reverse)
    (:Update
      (Transformation|SetRelativeRotation (Variables|Default|GetDoorHinge) (Math|Rotator|MakeRotator 0.0 0.0 (Math|Float|Lerp 0.0 9e+01 _opendoor)) false false))))

(event EventBeginPlay
  (if (Utilities|IsValidClass (Variables|Default|GetKeyActorClass))
    (bind _outactors (Actor|GetAllActorsOfClass (Variables|Default|GetKeyActorClass)))
    (Variables|Default|SetTotalKeys (Utilities|Array|Length _outactors))
    (for _array_element _outactors
      (EventDispatchers|BindEventtoKeyFound _array_element (delegate Custom|KeyFound)))
    (else
      (Variables|Default|SetCanOpen true))))

(fn ConstructionScript)