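; LockActor_BP is a lock that lights up when its paired key actor is found.
; The construction script gives the lock mesh a dynamic instance of the key mesh's material, so lock and key match visually.
; At BeginPlay it switches the material's Glow parameter off and binds to the key's KeyFound event, which raises Glow when fired.
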(event Custom|KeyFound
  (Rendering|Material|SetScalarParameterValue (Variables|Default|GetLockMaterial) "Glow" 1.2e+02 :!class /Script/Engine.MaterialInstanceDynamic))

(event EventBeginPlay
  (Rendering|Material|SetScalarParameterValue (Variables|Default|GetLockMaterial) "Glow" 0.0 :!class /Script/Engine.MaterialInstanceDynamic)
  (EventDispatchers|BindEventtoKeyFound (Variables|Default|GetKeyActor) (delegate Custom|KeyFound)))

(event Collision|EventActorBeginOverlap
  (params (OtherActor :type Actor%20Object%20Reference)))

(event EventTick
  (params (DeltaSeconds :type Float%20%28single-precision%29)))

(fn ConstructionScript
  ;[0.7176 0.5955 1] Set lock material to matching key material
  (bind _returnvalue (Rendering|Material|CreateDynamicMaterialInstance (Variables|Default|GetLockMesh) 0 (Rendering|Material|GetMaterial (Variables|/Game/Keys/KeyActorMASTER_BP.KeyActorMASTER_BP_C|GetKeyMesh (Variables|Default|GetKeyActor)) 0) "None" :!class /Script/Engine.PrimitiveComponent))
  (Variables|Default|SetLockMaterial _returnvalue))